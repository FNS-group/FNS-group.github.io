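; VR hand actor for a motion controller that grabs objects and aims teleports, with its tracking source set by the Hand variable.
; Grabbing picks the nearest PickupActorInterface actor overlapping its sphere and messages it to attach; releasing drops it only if still attached to this controller.
; While PressingTeleport is set, Tick runs a debug-drawn line trace from the arrow, validating hits on actors tagged WalkVolume as destinations.
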(event `self.ReceiveTick`
  (params (DeltaSeconds :type "Float (single-precision)"))
  (if (`self.bPressingTeleport`)
    (`self.TraceTeleportDestination`)))

(fn `GetActorNearHand`
  (returns (NearestActor :type "Actor Object Reference"))
  (locals (NearestOverlappingActor :type "Actor Object Reference") (NearestOverlap :type "Float (double-precision)" :default 1000.0))
  (bind _sphere (`self.Sphere`))
  (for _array_element (`PrimitiveComponent.GetOverlappingActors` _sphere "/Script/Engine.Actor")
    (if (`KismetSystemLibrary.DoesImplementInterface` _array_element "/Game/Blueprints/PickupActorInterface.PickupActorInterface_C")
      (bind _returnvalue (`KismetMathLibrary.VSize` (- (`self.K2_GetActorLocation` _array_element) (`SceneComponent.K2_GetComponentLocation` _sphere))))
      (if (< _returnvalue (`local.NearestOverlap`))
        (set `local.NearestOverlappingActor` _array_element)
        (set `local.NearestOverlap` _returnvalue))))
  (return (`local.NearestOverlappingActor`)))

(fn `GrabActor`
  (set `self.bWantsToGrip` true)
  (bind _nearestactor (`self.GetActorNearHand`))
  (`/Engine/EditorBlueprintResources/StandardMacros.IsValid` _nearestactor
    (:`Is Valid`
      (bind _output_get (set `self.AttachedActor` _nearestactor))
      (message `/Game/Blueprints/PickupActorInterface.PickUp` _output_get (`self.MotionController`)))))

(fn `ReleaseActor`
  (bind _attachedactor (`self.AttachedActor`))
  (set `self.bWantsToGrip` false)
  (`/Engine/EditorBlueprintResources/StandardMacros.IsValid` _attachedactor
    (:`Is Valid`
      (if (== (`SceneComponent.GetAttachParent` (`Actor.RootComponent` _attachedactor)) (`self.MotionController`))
        (message `/Game/Blueprints/PickupActorInterface.Drop` _attachedactor)))))

(fn `TraceTeleportDestination`
  (returns (bPointToValid :type Boolean) (PointingPosition :type "Vector Structure"))
  (locals (ValidLocation :type Boolean) (ValidPosition :type "Vector Structure"))
  (bind _arrow (`self.Arrow`))
  (bind _returnvalue (`SceneComponent.K2_GetComponentLocation` _arrow))
  (bind (_outhit _returnvalue_2) (`KismetSystemLibrary.LineTraceSingle` :`Start` _returnvalue :`End` (+ _returnvalue (* (`SceneComponent.GetForwardVector` _arrow) (`self.RayDistance`))) :`TraceChannel` "TraceTypeQuery1" :`DrawDebugType` "ForOneFrame" :`DrawTime` 2.0))
  (if _returnvalue_2
    (bind (_bblockinghit _binitialoverlap _time _distance _location _impactpoint _normal _impactnormal _physmat _hitactor) (`GameplayStatics.BreakHitResult` _outhit))
    (if (`self.ActorHasTag` _hitactor "WalkVolume")
      (set `local.ValidLocation` true)
      (set `local.ValidPosition` _impactpoint)
      (else
        (set `local.ValidLocation` false)
        (set `local.ValidPosition` (0.0 0.0 0.0))))
    (return (`local.ValidLocation`) (`local.ValidPosition`))))

(fn `UserConstructionScript`
  (set `MotionControllerComponent.MotionSource` (`|GetEnumeratorName` (`self.Hand`)) (`self.MotionController`)))